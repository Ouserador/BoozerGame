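; BP_Barrier is a level obstacle that changes its look per level and is removed when OpenBarrier destroys it.
; On BeginPlay it checks the current level name, showing the two bottle meshes everywhere except Level_2.
; In Level_4 it hides and disables collision on the main mesh and bottles, enabling the alternate BarrierLvl4 mesh instead.
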(event Custom|OpenBarrier
  (Actor|DestroyActor))

(event EventBeginPlay
  (bind _bottle_1 (Variables|Default|GetBottle_1))
  (bind _bottle_2 (Variables|Default|GetBottle_2))
  (bind _barrierlvl4 (Variables|Default|GetBarrierLvl4))
  (bind _barrierlvl4_2 (Variables|Default|GetBarrierLvl4))
  (bind _mesh (Variables|Default|GetMesh))
  (Rendering|SetVisibility _barrierlvl4_2 false false)
  (Collision|SetCollisionEnabled _barrierlvl4_2 "NoCollision")
  (Utilities|FlowControl|Sequence
    (:then_0
      (bind _returnvalue (Game|GetCurrentLevelName true))
      (Utilities|FlowControl|Sequence
        (:then_0
          (Rendering|SetVisibility (Variables|Default|GetBottle_1) (not (Utilities|Enum|Equal(Enum) _returnvalue "Level_2")) false))
        (:then_1
          (Rendering|SetVisibility (Variables|Default|GetBottle_2) (not (Utilities|Enum|Equal(Enum) _returnvalue "Level_2")) false))))
    (:then_1
      (bind _returnvalue_2 (Game|GetCurrentLevelName true))
      (if (Utilities|Enum|Equal(Enum) _returnvalue_2 "Level_4")
        (Utilities|FlowControl|Sequence
          (:then_0
            (Rendering|SetVisibility _bottle_1 false false)
            (Collision|SetCollisionEnabled _bottle_1 "NoCollision"))
          (:then_1
            (Rendering|SetVisibility _bottle_2 false false)
            (Collision|SetCollisionEnabled _bottle_2 "NoCollision"))
          (:then_2
            (Rendering|SetVisibility _mesh false false)
            (Collision|SetCollisionEnabled _mesh "NoCollision"))
          (:then_3
            (Rendering|SetVisibility _barrierlvl4 true false)
            (Collision|SetCollisionEnabled _barrierlvl4 "QueryAndPhysics")))))))

(fn ConstructionScript)