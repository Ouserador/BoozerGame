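; BP_DeathZone is a level hazard that kills the BP_Boozer character when it enters the zone's Box trigger.
; The overlap casts the game mode to GM_LevelManager and calls OnDying, leaving death handling to it.
; The mesh look follows the level name: lava in Level_3, water otherwise, set in both the construction script and BeginPlay.
; BeginPlay also hides the mesh in Level_4 and Level_5.
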(event OnComponentBeginOverlap(Box)
  (params (OverlappedComponent :type Primitive%20Component%20Object%20Reference) (OtherActor :type Actor%20Object%20Reference) (OtherComp :type Primitive%20Component%20Object%20Reference) (OtherBodyIndex :type Integer) (bFromSweep :type Boolean) (SweepResult :type Hit%20Result%20Structure%20%28by%20ref%29))
  ;[1 0 0] Death management
  (Utilities|Casting|CastToBP_Boozer OtherActor)
  (bind _asgm_level_manager (Utilities|Casting|CastToGM_LevelManager (Game|GetGameMode)))
  (Default|OnDying _asgm_level_manager))

(event EventBeginPlay
  (bind _mesh (Variables|Default|GetMesh))
  ;[0 0.5052 0.2109] Set material depending on the level
  (Utilities|FlowControl|Sequence
    (:then_0
      (bind _returnvalue (Game|GetCurrentLevelName true))
      (Rendering|SetVisibility (Variables|Default|GetMesh) (not (or (Utilities|Enum|Equal(Enum) _returnvalue "Level_4") (Utilities|Enum|Equal(Enum) _returnvalue "Level_5"))) false) ; Level 4 is on the clouds, so the mesh will be hidden.
    )
    (:then_1
      (bind _returnvalue_2 (Game|GetCurrentLevelName true))
      (if (Utilities|Enum|Equal(Enum) _returnvalue_2 "Level_3")
        (Rendering|Material|SetMaterial _mesh 0 "/Game/Materials/M_Lava.M_Lava")
        (else
          (Rendering|Material|SetMaterial _mesh 0 "/Game/Materials/M_Water.M_Water"))))))

(fn ConstructionScript
  (bind _mesh (Variables|Default|GetMesh))
  (bind _returnvalue (Game|GetCurrentLevelName true))
  (if (Utilities|Enum|Equal(Enum) _returnvalue "Level_3")
    (Rendering|Material|SetMaterial _mesh 0 "/Game/Materials/M_Lava.M_Lava")
    (else
      (Rendering|Material|SetMaterial _mesh 0 "/Game/Materials/M_Water.M_Water"))))