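; Tutorial poster placed in levels that shows a paused, full UI tutorial for its selected TutorialType.
; The construction script and BeginPlay pick the matching poster material, and a timeline animates the mesh's height.
; Its trigger zone registers the poster with BP_Boozer as the nearest interactable and toggles a button pop-up.
; ShowTutorial creates the tutorial manager widget with the matching image, pauses the game and switches to UI-only input.
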(event OnComponentBeginOverlap(TriggerZone)
  (params (OverlappedComponent :type Primitive%20Component%20Object%20Reference) (OtherActor :type Actor%20Object%20Reference) (OtherComp :type Primitive%20Component%20Object%20Reference) (OtherBodyIndex :type Integer) (bFromSweep :type Boolean) (SweepResult :type Hit%20Result%20Structure%20%28by%20ref%29))
  ;[0 0.04299 0.5] Collision detection and pop-up UI
  (bind _asbp_boozer (Utilities|Casting|CastToBP_Boozer OtherActor))
  (Variables|/Game/Blueprints/BP_Boozer.BP_Boozer_C|SetcanInteract _asbp_boozer true)
  (Variables|/Game/Blueprints/BP_Boozer.BP_Boozer_C|SetinteractionType _asbp_boozer "NewEnumerator6")
  (Variables|/Game/Blueprints/BP_Boozer.BP_Boozer_C|SetnearestTutorialPoster _asbp_boozer self)
  (Rendering|SetVisibility (Variables|Default|GetButtonPopUp) true false))

(event OnComponentEndOverlap(TriggerZone)
  (params (OverlappedComponent :type Primitive%20Component%20Object%20Reference) (OtherActor :type Actor%20Object%20Reference) (OtherComp :type Primitive%20Component%20Object%20Reference) (OtherBodyIndex :type Integer))
  ;[0 0.04299 0.5] Collision detection and pop-up UI
  (bind _asbp_boozer (Utilities|Casting|CastToBP_Boozer OtherActor))
  (Variables|/Game/Blueprints/BP_Boozer.BP_Boozer_C|SetcanInteract _asbp_boozer false)
  (Variables|/Game/Blueprints/BP_Boozer.BP_Boozer_C|SetinteractionType _asbp_boozer "NewEnumerator0")
  (Rendering|SetVisibility (Variables|Default|GetButtonPopUp) false false))

(event EventBeginPlay
  (bind _buttonpopup (Variables|Default|GetButtonPopUp))
  (bind _mesh (Variables|Default|GetMesh))
  (Utilities|FlowControl|Sequence
    (:then_0
      (switch Utilities|FlowControl|Switch|SwitchonTutorialType (Variables|Default|GettutorialType) ; Set the material with the corresponding image.
        (:NewEnumerator0
          (Rendering|Material|SetMaterial _mesh 0 "/Game/Materials/Poster/M_Poster_Movement.M_Poster_Movement"))
        (:NewEnumerator5
          (Rendering|Material|SetMaterial _mesh 0 "/Game/Materials/Poster/MI_Poster_VisionType.MI_Poster_VisionType"))
        (:NewEnumerator1
          (Rendering|Material|SetMaterial _mesh 0 "/Game/Materials/Poster/MI_Poster_AbilityColor.MI_Poster_AbilityColor"))
        (:NewEnumerator2
          (Rendering|Material|SetMaterial _mesh 0 "/Game/Materials/Poster/MI_Poster_DoorManager.MI_Poster_DoorManager"))
        (:NewEnumerator3
          (Rendering|Material|SetMaterial _mesh 0 "/Game/Materials/Poster/MI_Poster_PurplePlatforms.MI_Poster_PurplePlatforms"))
        (:NewEnumerator6
          (Rendering|Material|SetMaterial _mesh 0 "/Game/Materials/Poster/MI_Poster_ObstacleSlower.MI_Poster_ObstacleSlower"))
        (:NewEnumerator7
          (Rendering|Material|SetMaterial _mesh 0 "/Game/Materials/Poster/MI_Poster_PlatformMover.MI_Poster_PlatformMover"))))
    (:then_1
      (Rendering|SetVisibility _buttonpopup false false)
      (bind _asui_stone (Utilities|Casting|CastToUI_Stone (UserInterface|GetWidget _buttonpopup)))
      (Default|IsInteractionAvailable _asui_stone true))
    (:then_2
      (bind _posz (Timeline|Timeline Play)
        (:Update
          (Transformation|SetRelativeLocation (Variables|Default|GetMesh) (Math|Vector|MakeVector 0.0 0.0 _posz) false false) ; The arrow will move in its default position.
        )))))

(fn ConstructionScript
  (bind _mesh (Variables|Default|GetMesh))
  (switch Utilities|FlowControl|Switch|SwitchonTutorialType (Variables|Default|GettutorialType)
    (:NewEnumerator0
      (Rendering|Material|SetMaterial _mesh 0 "/Game/Materials/Poster/M_Poster_Movement.M_Poster_Movement"))
    (:NewEnumerator5
      (Rendering|Material|SetMaterial _mesh 0 "/Game/Materials/Poster/MI_Poster_VisionType.MI_Poster_VisionType"))
    (:NewEnumerator1
      (Rendering|Material|SetMaterial _mesh 0 "/Game/Materials/Poster/MI_Poster_AbilityColor.MI_Poster_AbilityColor"))
    (:NewEnumerator2
      (Rendering|Material|SetMaterial _mesh 0 "/Game/Materials/Poster/MI_Poster_DoorManager.MI_Poster_DoorManager"))
    (:NewEnumerator3
      (Rendering|Material|SetMaterial _mesh 0 "/Game/Materials/Poster/MI_Poster_PurplePlatforms.MI_Poster_PurplePlatforms"))
    (:NewEnumerator6
      (Rendering|Material|SetMaterial _mesh 0 "/Game/Materials/Poster/MI_Poster_ObstacleSlower.MI_Poster_ObstacleSlower"))
    (:NewEnumerator7
      (Rendering|Material|SetMaterial _mesh 0 "/Game/Materials/Poster/MI_Poster_PlatformMover.MI_Poster_PlatformMover"))))

(fn ShowTutorial
  (bind _returnvalue (Game|GetPlayerController 0))
  (bind _returnvalue_2 (UserInterface|CreateWidget "/Game/UI/UI_TutorialManager.UI_TutorialManager_C"))
  (bind _output_get (Variables|Default|SettutorialUI _returnvalue_2))
  (Default|UpdateTutorialImg _output_get (Variables|Default|GettutorialType))
  (UserInterface|Viewport|AddtoViewport _output_get 0)
  (Game|SetGamePaused true)
  (Input|SetInputModeUIOnly _returnvalue 0 "DoNotLock" false)
  (Variables|/Script/Engine.PlayerController|SetbShowMouseCursor _returnvalue true))