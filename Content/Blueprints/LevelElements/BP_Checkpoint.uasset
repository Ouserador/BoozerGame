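; BP_Checkpoint is a level element that records the player's progress when a BP_Boozer passes through it.
; While active, its PassZone overlap fires once, storing the Boozer manager's current color and setting the Boozer's current checkpoint to its own value.
; It then shows the checkpoint-reached HUD text and, if allowed, activates the linked next checkpoint, forming a chain.
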(event OnComponentBeginOverlap(PassZone)
  (params (OverlappedComponent :type Primitive%20Component%20Object%20Reference) (OtherActor :type Actor%20Object%20Reference) (OtherComp :type Primitive%20Component%20Object%20Reference) (OtherBodyIndex :type Integer) (bFromSweep :type Boolean) (SweepResult :type Hit%20Result%20Structure%20%28by%20ref%29))
  (if (Variables|Default|GetisActive)
    (if (not (Variables|Default|GetboozerHasPassed)) ; Executes once.
      (bind _asbp_boozer (Utilities|Casting|CastToBP_Boozer OtherActor))
      (Variables|Default|SetcolorType (Variables|/Game/Blueprints/GameModes/GM_LevelManager.GM_LevelManager_C|GetcurrentColor (Variables|/Game/Blueprints/BP_Boozer.BP_Boozer_C|Getmanager _asbp_boozer)))
      (Variables|/Game/Blueprints/BP_Boozer.BP_Boozer_C|SetcurrentCheckpoint _asbp_boozer (Variables|Default|GetcheckPointValue))
      (Variables|Default|SetboozerHasPassed true)
      (Default|CheckpointReachedTxt (Variables|/Game/Blueprints/GameModes/GM_LevelManager.GM_LevelManager_C|GetplayerHUD (Variables|/Game/Blueprints/BP_Boozer.BP_Boozer_C|Getmanager _asbp_boozer)))
      (if (Variables|Default|GetcanSpawnCheckpoint)
        (Variables|BP_Checkpoint_C|SetisActive (Variables|Default|GetnewCheckpoint) true)))))

(fn ConstructionScript)