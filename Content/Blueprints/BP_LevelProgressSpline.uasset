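; BP_LevelProgressSpline is a level actor that measures BP_Boozer's progress along the level for the HUD progress bar.
; It finds the Boozer at BeginPlay, then each tick copies that actor's world X into RefPoint's relative X.
; That value, clamped to the spline's length and normalized to 0–1, goes to PlayerHUD's UpdateProgress via the Boozer's Manager.
; The spline supplies only its length, so progress is measured along X alone.
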(event EventBeginPlay
  (bind _returnvalue (Actor|GetActorOfClass "/Game/Blueprints/BP_Boozer.BP_Boozer_C"))
  (Variables|Default|SetboozerObj _returnvalue))

(event EventTick
  (params (DeltaSeconds :type Float%20%28single-precision%29))
  (bind _refpoint (Variables|Default|GetRefPoint))
  (bind _relativelocation (Variables|/Script/Engine.SceneComponent|GetRelativeLocation _refpoint))
  (Transformation|SetRelativeLocation (Variables|Default|GetRefPoint) (Math|Vector|MakeVector (.x (Transformation|GetActorLocation (Variables|Default|GetboozerObj))) (.y _relativelocation) (.z _relativelocation)) false false)
  (Default|UpdateProgress (Variables|/Game/Blueprints/GameModes/GM_LevelManager.GM_LevelManager_C|GetplayerHUD (Variables|/Game/Blueprints/BP_Boozer.BP_Boozer_C|Getmanager (Variables|Default|GetboozerObj))) (/ (Math|Float|Clamp(Float) (.x _relativelocation) 0.0 (Spline|GetSplineLength (Variables|Default|GetSpline))) (Spline|GetSplineLength (Variables|Default|GetSpline)))))

(fn ConstructionScript)