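; Game Instance Blueprint that holds the colorblind mode and strength and applies them as color vision deficiency settings.
; SetValues stores both values, then switches on the type to call SetColorVisionDeficiencyType for normal vision, deuteranope, protanope or tritanope.
; Every call enables both correction and showing the correction with the deficiency simulated.
; GetValues returns the stored type and strength.
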(fn SetValues
  (params (currentColorBlind :type ColorBlindType%20Enum :default "NewEnumerator0") (currentStrenght :type Float%20%28double-precision%29))
  (Variables|Default|SetcbStrenght currentStrenght)
  (bind _output_get (Variables|Default|SetcbType currentColorBlind))
  (switch Utilities|FlowControl|Switch|SwitchonColorBlindType _output_get
    (:NewEnumerator0
      (Class|WidgetBlueprintLibrary|SetColorVisionDeficiencyType "NormalVision" (Variables|Default|GetcbStrenght) true true))
    (:NewEnumerator1
      (Class|WidgetBlueprintLibrary|SetColorVisionDeficiencyType "Deuteranope" (Variables|Default|GetcbStrenght) true true))
    (:NewEnumerator2
      (Class|WidgetBlueprintLibrary|SetColorVisionDeficiencyType "Protanope" (Variables|Default|GetcbStrenght) true true))
    (:NewEnumerator3
      (Class|WidgetBlueprintLibrary|SetColorVisionDeficiencyType "Tritanope" (Variables|Default|GetcbStrenght) true true))))

(fn GetValues
  (return (Variables|Default|GetcbType) (Variables|Default|GetcbStrenght)))