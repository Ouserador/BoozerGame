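; Colored platform actor that can optionally travel along a referenced spline path.
; Construction applies the grey, red or blue material with collision enabled and snaps movable platforms to the spline's first point.
; At BeginPlay, a timeline scaled by TimeBeforeTurn lerps distance along the spline, keeping the start point's local rotation.
; Each update re-triggers movement while IsMovable holds, otherwise stops the timeline.
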(event Custom|MovePlatformThroughSpline
  (bind _splinepath (Variables|Main|GetsplinePath))
  (bind _spline (Variables|/Game/Blueprints/BP_Spline.BP_Spline_C|GetSpline _splinepath))
  (Components|Timeline|SetPlayRate (Variables|Default|GetMovementInterp) (/ 1.0 (Variables|Movement|GettimeBeforeTurn)))
  (bind _newtrack_0 (Timeline|MovementInterp Play)
    (:Update
      (Transformation|SetActorTransform (Math|Transform|MakeTransform (Spline|GetLocationatDistanceAlongSpline _spline (Math|Float|Lerp 0.0 (Spline|GetSplineLength _spline) _newtrack_0) "World") (Spline|GetRotationatDistanceAlongSpline _spline 0.0 "Local") "1.000000,1.000000,1.000000"))
      (if (Variables|Main|GetisMovable)
        (CallFunction|MovePlatformThroughSpline)
        (else
          (Audio|Components|Audio|Stop (Variables|Default|GetMovementInterp)))))))

(event EventBeginPlay
  (if (Variables|Main|GetisMovable)
    (CallFunction|MovePlatformThroughSpline)))

(fn ConstructionScript
  (Utilities|FlowControl|Sequence
    (:then_0
      (CallFunction|UpdateColor (Variables|Main|GetcurrentColor)))
    (:then_1
      (if (Variables|Main|GetisMovable)
        (Transformation|SetActorLocation (Spline|GetLocationatSplinePoint (Variables|/Game/Blueprints/BP_Spline.BP_Spline_C|GetSpline (Variables|Main|GetsplinePath)) 0 "World") false false)))))

(fn UpdateColor
  (params (newColor :type PlatformColor%20Enum :default "NewEnumerator0"))
  (switch Utilities|FlowControl|Switch|SwitchonPlatformColor newColor
    (:NewEnumerator0
      (CallFunction|ChangeProperties "/Game/Materials/_TESTING/MI_Grey.MI_Grey" true))
    (:NewEnumerator1
      (CallFunction|ChangeProperties "/Game/Materials/_TESTING/MI_Red.MI_Red" true))
    (:NewEnumerator2
      (CallFunction|ChangeProperties "/Game/Materials/_TESTING/MI_Blue.MI_Blue" true))))

(fn ChangeProperties
  (params (newColorMat :type Material%20Interface%20Object%20Reference) (hasCollision :type Boolean))
  (bind _mesh (Variables|Default|GetMesh))
  (Utilities|FlowControl|Sequence
    (:then_0
      (Rendering|Material|SetMaterial (Variables|Default|GetMesh) 0 newColorMat) ; Change material.
    )
    (:then_1
      (if hasCollision
        (Collision|SetCollisionEnabled _mesh "QueryAndPhysics")
        (Variables|Default|SetisTransparent false)
        (else
          (Collision|SetCollisionEnabled _mesh "NoCollision")
          (Variables|Default|SetisTransparent true))))))