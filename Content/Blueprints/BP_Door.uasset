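; Colored door actor, green or yellow, that can switch between a solid state and a transparent, passable state.
; The construction script applies the solid material matching CurrentColor to the Door mesh.
; AlterProperties takes a transparency flag and color, then toggles the door's collision and swaps to the matching solid or transparent material.
; The event graph holds no logic, and nothing in this Blueprint calls AlterProperties.
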(event EventBeginPlay)

(event Collision|EventActorBeginOverlap
  (params (OtherActor :type Actor%20Object%20Reference)))

(event EventTick
  (params (DeltaSeconds :type Float%20%28single-precision%29)))

(fn ConstructionScript
  (bind _door (Variables|Default|GetDoor))
  (switch Utilities|FlowControl|Switch|SwitchonDoorColor (Variables|Default|GetcurrentColor)
    (:NewEnumerator0
      (Rendering|Material|SetMaterial _door 0 "/Game/Materials/_TESTING/MI_DoorGreen.MI_DoorGreen"))
    (:NewEnumerator1
      (Rendering|Material|SetMaterial _door 0 "/Game/Materials/_TESTING/MI_DoorYellow.MI_DoorYellow"))))

(fn AlterProperties
  (params (isTransparent :type Boolean) (doorColor :type DoorColor%20Enum :default "NewEnumerator0"))
  (if isTransparent
    (Collision|SetCollisionEnabled (Variables|Default|GetDoor) "NoCollision")
    (switch Utilities|FlowControl|Switch|SwitchonDoorColor doorColor
      (:NewEnumerator0
        (Rendering|Material|SetMaterial (Variables|Default|GetDoor) 0 "/Game/Materials/_TESTING/MI_DoorTransparentGreen.MI_DoorTransparentGreen"))
      (:NewEnumerator1
        (Rendering|Material|SetMaterial (Variables|Default|GetDoor) 0 "/Game/Materials/_TESTING/MI_DoorTransparentYellow.MI_DoorTransparentYellow")))
    (else
      (Collision|SetCollisionEnabled (Variables|Default|GetDoor) "QueryAndPhysics")
      (switch Utilities|FlowControl|Switch|SwitchonDoorColor doorColor
        (:NewEnumerator0
          (Rendering|Material|SetMaterial (Variables|Default|GetDoor) 0 "/Game/Materials/_TESTING/MI_DoorGreen.MI_DoorGreen"))
        (:NewEnumerator1
          (Rendering|Material|SetMaterial (Variables|Default|GetDoor) 0 "/Game/Materials/_TESTING/MI_DoorYellow.MI_DoorYellow"))))))