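; Stone pillar timer that temporarily makes its linked purple platforms solid for the player (BP_Boozer).
; Its interaction zone registers it as the player's nearest timer; activation swaps platform materials, enables collision and lights the stone.
; Tick drives the HUD countdown, then restores translucent, non-colliding platforms when time runs out.
; Debug-drawn line traces link stone to platforms in normal vision and at construction.
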(event OnComponentBeginOverlap(InteractionZone)
  (params (OverlappedComponent :type Primitive%20Component%20Object%20Reference) (OtherActor :type Actor%20Object%20Reference) (OtherComp :type Primitive%20Component%20Object%20Reference) (OtherBodyIndex :type Integer) (bFromSweep :type Boolean) (SweepResult :type Hit%20Result%20Structure%20%28by%20ref%29))
  ;[1 1 1] Collision detector
  (bind _asbp_boozer (Utilities|Casting|CastToBP_Boozer OtherActor))
  (Variables|/Game/Blueprints/BP_Boozer.BP_Boozer_C|SetcanInteract _asbp_boozer true)
  (Variables|/Game/Blueprints/BP_Boozer.BP_Boozer_C|SetinteractionType _asbp_boozer "NewEnumerator1")
  (Variables|/Game/Blueprints/BP_Boozer.BP_Boozer_C|SetnearestTimer _asbp_boozer self))

(event OnComponentEndOverlap(InteractionZone)
  (params (OverlappedComponent :type Primitive%20Component%20Object%20Reference) (OtherActor :type Actor%20Object%20Reference) (OtherComp :type Primitive%20Component%20Object%20Reference) (OtherBodyIndex :type Integer))
  ;[1 1 1] Collision detector
  (bind _asbp_boozer (Utilities|Casting|CastToBP_Boozer OtherActor))
  (Variables|/Game/Blueprints/BP_Boozer.BP_Boozer_C|SetcanInteract _asbp_boozer false)
  (Variables|/Game/Blueprints/BP_Boozer.BP_Boozer_C|SetinteractionType _asbp_boozer "NewEnumerator0"))

(event Custom|ActivePurplePlatformTimer
  ;[0.0322 0 0.09375] Platform timer
  (if (not (Variables|Default|GetisActive))
    (for _array_element (Variables|Default|GetpurplePlatforms)
      (Default|ChangeProperties _array_element "/Game/Materials/Platforms/MI_Platform_Purple.MI_Platform_Purple" true))
    (Variables|Default|SetticTac true)
    (Rendering|Material|SetMaterial (Variables|Default|GetStone) 0 "/Game/Materials/StonePilars/M_StonePilar_Purple_On.M_StonePilar_Purple_On")
    (Default|TimerShowing (Variables|/Game/Blueprints/GameModes/GM_LevelManager.GM_LevelManager_C|GetplayerHUD (Variables|/Game/Blueprints/BP_Boozer.BP_Boozer_C|Getmanager (Variables|Default|GetboozerObj))) true)))

(event EventBeginPlay
  (Utilities|FlowControl|Sequence
    (:then_0
      (bind _returnvalue (Actor|GetActorOfClass "/Game/Blueprints/BP_Boozer.BP_Boozer_C"))
      (Variables|Default|SetboozerObj _returnvalue))
    (:then_1
      (Variables|Default|Settimer (Variables|Default|GettimeBeforeInactive)))))

(event EventTick
  (params (DeltaSeconds :type Float%20%28single-precision%29))
  (bind _debugcolor (Variables|Default|GetdebugColor))
  (Utilities|FlowControl|Sequence
    (:then_0
      ;[0.1838 0 0.3229] Pointer
      (switch Utilities|FlowControl|Switch|SwitchonVisionType (Variables|/Game/Blueprints/BP_Boozer.BP_Boozer_C|GetcurrentVisionType (Variables|Default|GetboozerObj))
        (:NewEnumerator0
          (for _array_element (Variables|Default|GetpurplePlatforms)
            (switch Utilities|FlowControl|Switch|SwitchonPlatformColor (Variables|/Game/Blueprints/GameLlements/BP_Platform.BP_Platform_C|GetcurrentColor _array_element)
              (:NewEnumerator2
                _)
              (:NewEnumerator3
                _))
            (Collision|LineTraceByChannel (+ (Transformation|GetWorldLocation (Variables|Default|GetStone)) (Math|Vector|MakeVector 0.0 0.0 2e+01)) (Transformation|GetActorLocation _array_element) "TraceTypeQuery1" false 0 "ForOneFrame" true _debugcolor _debugcolor)))))
    (:then_1
      ;[0.0322 0 0.09375] Platform timer
      (if (Variables|Default|GetticTac)
        (bind _output_get (Variables|Default|Settimer (- (Variables|Default|Gettimer) (Utilities|Time|GetWorldDeltaSeconds))))
        (Default|TimerBehaviour (Variables|/Game/Blueprints/GameModes/GM_LevelManager.GM_LevelManager_C|GetplayerHUD (Variables|/Game/Blueprints/BP_Boozer.BP_Boozer_C|Getmanager (Variables|Default|GetboozerObj))) (/ _output_get (Variables|Default|GettimeBeforeInactive)))
        (if (<= (Variables|Default|Gettimer) 0.0)
          (for _array_element_2 (Variables|Default|GetpurplePlatforms)
            (Default|ChangeProperties _array_element_2 "/Game/Materials/Platforms/M_PlatformTranslucent_Purple.M_PlatformTranslucent_Purple" false))
          (Rendering|Material|SetMaterial (Variables|Default|GetStone) 0 "/Game/Materials/StonePilars/M_StonePilar_Off.M_StonePilar_Off")
          (Variables|Default|SetisActive false)
          (Variables|Default|SetticTac false)
          (bind _output_get_2 (Variables|Default|Settimer (Variables|Default|GettimeBeforeInactive)))
          (Default|TimerBehaviour (Variables|/Game/Blueprints/GameModes/GM_LevelManager.GM_LevelManager_C|GetplayerHUD (Variables|/Game/Blueprints/BP_Boozer.BP_Boozer_C|Getmanager (Variables|Default|GetboozerObj))) (/ _output_get_2 (Variables|Default|GettimeBeforeInactive)))
          (Default|TimerShowing (Variables|/Game/Blueprints/GameModes/GM_LevelManager.GM_LevelManager_C|GetplayerHUD (Variables|/Game/Blueprints/BP_Boozer.BP_Boozer_C|Getmanager (Variables|Default|GetboozerObj))) false))))
    (:then_2)))

(fn ConstructionScript
  (for _array_element (Variables|Default|GetpurplePlatforms)
    (switch Utilities|FlowControl|Switch|SwitchonPlatformColor (Variables|/Game/Blueprints/GameLlements/BP_Platform.BP_Platform_C|GetcurrentColor _array_element)
      (:NewEnumerator3
        (Collision|LineTraceByChannel (+ (Transformation|GetWorldLocation (Variables|Default|GetStone)) (Math|Vector|MakeVector 0.0 0.0 2e+01)) (Transformation|GetActorLocation _array_element) "TraceTypeQuery1" false 0 "ForDuration" true "(R=1.000000,G=0.000000,B=0.588235,A=1.000000)" "(R=1.000000,G=0.000000,B=0.588235,A=1.000000)")))))