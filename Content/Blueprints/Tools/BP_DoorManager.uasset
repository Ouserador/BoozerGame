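; BP_DoorManager is a switch actor that controls a set of green and yellow doors, starting green doors non-transparent and yellow doors transparent.
; Invert flips a boolean and reapplies transparency so the two colors stay opposite.
; Its InteractionZone overlap enables interaction on BP_Boozer and registers itself as the nearest manager.
; Construction Script and Tick use line traces with persistent debug drawing to show color-coded links to each door.
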(event OnComponentBeginOverlap(InteractionZone)
  (params (OverlappedComponent :type Primitive%20Component%20Object%20Reference) (OtherActor :type Actor%20Object%20Reference) (OtherComp :type Primitive%20Component%20Object%20Reference) (OtherBodyIndex :type Integer) (bFromSweep :type Boolean) (SweepResult :type Hit%20Result%20Structure%20%28by%20ref%29))
  (bind _asbp_boozer (Utilities|Casting|CastToBP_Boozer OtherActor))
  (Variables|/Game/Blueprints/BP_Boozer.BP_Boozer_C|SetcanInteract _asbp_boozer true)
  (Variables|/Game/Blueprints/BP_Boozer.BP_Boozer_C|SetinteractionType _asbp_boozer "NewEnumerator4")
  (Variables|/Game/Blueprints/BP_Boozer.BP_Boozer_C|SetnearestDoorManager _asbp_boozer self))

(event OnComponentEndOverlap(InteractionZone)
  (params (OverlappedComponent :type Primitive%20Component%20Object%20Reference) (OtherActor :type Actor%20Object%20Reference) (OtherComp :type Primitive%20Component%20Object%20Reference) (OtherBodyIndex :type Integer))
  (bind _asbp_boozer (Utilities|Casting|CastToBP_Boozer OtherActor))
  (Variables|/Game/Blueprints/BP_Boozer.BP_Boozer_C|SetcanInteract _asbp_boozer false)
  (Variables|/Game/Blueprints/BP_Boozer.BP_Boozer_C|SetinteractionType _asbp_boozer "NewEnumerator0"))

(event EventTick
  (params (DeltaSeconds :type Float%20%28single-precision%29))
  (bind _returnvalue (Transformation|GetActorLocation))
  (for _array_element (Variables|Default|GetnumDoors)
    (switch Utilities|FlowControl|Switch|SwitchonDoorColor (Variables|/Game/Blueprints/BP_Door.BP_Door_C|GetcurrentColor _array_element)
      (:NewEnumerator0
        (Collision|LineTraceByChannel _returnvalue (Transformation|GetActorLocation _array_element) "TraceTypeQuery1" false 0 "Persistent" true "(R=0.001142,G=1.000000,B=0.000000,A=1.000000)" "(R=0.001214,G=1.000000,B=0.000000,A=1.000000)"))
      (:NewEnumerator1
        (Collision|LineTraceByChannel _returnvalue (Transformation|GetActorLocation _array_element) "TraceTypeQuery1" false 0 "Persistent" true "(R=0.996746,G=1.000000,B=0.000000,A=1.000000)" "(R=1.000000,G=1.000000,B=0.000000,A=1.000000)")))))

(event EventBeginPlay
  (for _array_element (Variables|Default|GetnumDoors)
    (switch Utilities|FlowControl|Switch|SwitchonDoorColor (Variables|/Game/Blueprints/BP_Door.BP_Door_C|GetcurrentColor _array_element)
      (:NewEnumerator0
        (Default|AlterProperties _array_element false "NewEnumerator0"))
      (:NewEnumerator1
        (Default|AlterProperties _array_element true "NewEnumerator1")))))

(fn ConstructionScript
  (bind _returnvalue (Transformation|GetActorLocation))
  (for _array_element (Variables|Default|GetnumDoors)
    (switch Utilities|FlowControl|Switch|SwitchonDoorColor (Variables|/Game/Blueprints/BP_Door.BP_Door_C|GetcurrentColor _array_element)
      (:NewEnumerator0
        (Collision|LineTraceByChannel _returnvalue (Transformation|GetActorLocation _array_element) "TraceTypeQuery1" false 0 "Persistent" true "(R=0.001142,G=1.000000,B=0.000000,A=1.000000)" "(R=0.001214,G=1.000000,B=0.000000,A=1.000000)"))
      (:NewEnumerator1
        (Collision|LineTraceByChannel _returnvalue (Transformation|GetActorLocation _array_element) "TraceTypeQuery1" false 0 "Persistent" true "(R=0.996746,G=1.000000,B=0.000000,A=1.000000)" "(R=1.000000,G=1.000000,B=0.000000,A=1.000000)")))))

(fn Invert
  (Variables|Default|SetisInverted (not (Variables|Default|GetisInverted)))
  (for _array_element (Variables|Default|GetnumDoors)
    (switch Utilities|FlowControl|Switch|SwitchonDoorColor (Variables|/Game/Blueprints/BP_Door.BP_Door_C|GetcurrentColor _array_element)
      (:NewEnumerator0
        (Default|AlterProperties _array_element (Variables|Default|GetisInverted) "NewEnumerator0"))
      (:NewEnumerator1
        (Default|AlterProperties _array_element (not (Variables|Default|GetisInverted)) "NewEnumerator1")))))