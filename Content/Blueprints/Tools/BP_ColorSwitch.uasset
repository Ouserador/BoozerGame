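; BP_ColorSwitch is an interactable stone pillar that toggles the level's current color between red and blue.
; Its overlap zone flags BP_Boozer as able to interact and registers itself as the nearest switch.
; The pillar material mirrors GM_LevelManager's color at BeginPlay and first Tick.
; SwitchBoozerColor flips that color, then has the manager refresh platform translucency by Boozer's vision type and update Boozer's color.
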(event OnComponentBeginOverlap(InteractionZone)
  (params (OverlappedComponent :type Primitive%20Component%20Object%20Reference) (OtherActor :type Actor%20Object%20Reference) (OtherComp :type Primitive%20Component%20Object%20Reference) (OtherBodyIndex :type Integer) (bFromSweep :type Boolean) (SweepResult :type Hit%20Result%20Structure%20%28by%20ref%29))
  (bind _asbp_boozer (Utilities|Casting|CastToBP_Boozer OtherActor))
  (Variables|/Game/Blueprints/BP_Boozer.BP_Boozer_C|SetcanInteract _asbp_boozer true)
  (Variables|/Game/Blueprints/BP_Boozer.BP_Boozer_C|SetinteractionType _asbp_boozer "NewEnumerator5")
  (Variables|/Game/Blueprints/BP_Boozer.BP_Boozer_C|SetnearestColorSwitch _asbp_boozer self))

(event OnComponentEndOverlap(InteractionZone)
  (params (OverlappedComponent :type Primitive%20Component%20Object%20Reference) (OtherActor :type Actor%20Object%20Reference) (OtherComp :type Primitive%20Component%20Object%20Reference) (OtherBodyIndex :type Integer))
  (bind _asbp_boozer (Utilities|Casting|CastToBP_Boozer OtherActor))
  (Variables|/Game/Blueprints/BP_Boozer.BP_Boozer_C|SetcanInteract _asbp_boozer false)
  (Variables|/Game/Blueprints/BP_Boozer.BP_Boozer_C|SetinteractionType _asbp_boozer "NewEnumerator0"))

(event EventBeginPlay
  (Utilities|FlowControl|Sequence
    (:then_0
      (bind _returnvalue (Actor|GetActorOfClass "/Game/Blueprints/BP_Boozer.BP_Boozer_C"))
      (Variables|Default|SetboozerObj _returnvalue))
    (:then_1
      (bind _asgm_level_manager (Utilities|Casting|CastToGM_LevelManager (Game|GetGameMode)))
      (bind _output_get (Variables|Default|Setmanager _asgm_level_manager))
      (switch Utilities|FlowControl|Switch|SwitchonColorType (Variables|/Game/Blueprints/GameModes/GM_LevelManager.GM_LevelManager_C|GetcurrentColor _output_get)
        (:NewEnumerator0
          (Rendering|Material|SetMaterial (Variables|Default|GetStone) 0 "/Game/Materials/StonePilars/MI_StonePilar_RED.MI_StonePilar_RED"))
        (:NewEnumerator1
          (Rendering|Material|SetMaterial (Variables|Default|GetStone) 0 "/Game/Materials/StonePilars/MI_StonePilar_BLUE.MI_StonePilar_BLUE"))))))

(event EventTick
  (params (DeltaSeconds :type Float%20%28single-precision%29))
  (if (Variables|Default|GetfirstTime)
    (Variables|Default|SetfirstTime false)
    (switch Utilities|FlowControl|Switch|SwitchonColorType (Variables|/Game/Blueprints/GameModes/GM_LevelManager.GM_LevelManager_C|GetcurrentColor (Variables|Default|Getmanager))
      (:NewEnumerator0
        (Rendering|Material|SetMaterial (Variables|Default|GetStone) 0 "/Game/Materials/StonePilars/MI_StonePilar_RED.MI_StonePilar_RED")
        (Variables|/Game/Blueprints/GameModes/GM_LevelManager.GM_LevelManager_C|SetisRedColor (Variables|Default|Getmanager) true))
      (:NewEnumerator1
        (Rendering|Material|SetMaterial (Variables|Default|GetStone) 0 "/Game/Materials/StonePilars/MI_StonePilar_BLUE.MI_StonePilar_BLUE")
        (Variables|/Game/Blueprints/GameModes/GM_LevelManager.GM_LevelManager_C|SetisRedColor (Variables|Default|Getmanager) false)))))

(fn ConstructionScript)

(fn SwitchBoozerColor
  (params (currentColor :type ColorType%20Enum :default "NewEnumerator0"))
  (bind _manager (Variables|Default|Getmanager))
  (bind _manager_2 (Variables|Default|Getmanager))
  (switch Utilities|FlowControl|Switch|SwitchonColorType currentColor
    (:NewEnumerator0
      (Rendering|Material|SetMaterial (Variables|Default|GetStone) 0 "/Game/Materials/StonePilars/MI_StonePilar_BLUE.MI_StonePilar_BLUE")
      (Variables|/Game/Blueprints/GameModes/GM_LevelManager.GM_LevelManager_C|SetisRedColor (Variables|Default|Getmanager) false))
    (:NewEnumerator1
      (Rendering|Material|SetMaterial (Variables|Default|GetStone) 0 "/Game/Materials/StonePilars/MI_StonePilar_RED.MI_StonePilar_RED")
      (Variables|/Game/Blueprints/GameModes/GM_LevelManager.GM_LevelManager_C|SetisRedColor (Variables|Default|Getmanager) true)))
  (switch Utilities|FlowControl|Switch|SwitchonColorType currentColor
    (:NewEnumerator0
      (Variables|/Game/Blueprints/GameModes/GM_LevelManager.GM_LevelManager_C|SetcurrentColor (Variables|Default|Getmanager) "NewEnumerator1"))
    (:NewEnumerator1
      (Variables|/Game/Blueprints/GameModes/GM_LevelManager.GM_LevelManager_C|SetcurrentColor (Variables|Default|Getmanager) "NewEnumerator0")))
  (switch Utilities|FlowControl|Switch|SwitchonVisionType (Variables|/Game/Blueprints/BP_Boozer.BP_Boozer_C|GetcurrentVisionType (Variables|Default|GetboozerObj))
    (:NewEnumerator0
      (Default|UpdatePlatformsBehaviour _manager_2 true true)
      (Default|UpdatePlatformsBehaviour _manager_2 false true))
    (:NewEnumerator1
      (Default|UpdatePlatformsBehaviour _manager_2 true false)
      (Default|UpdatePlatformsBehaviour _manager_2 false true))
    (:NewEnumerator2
      (Default|UpdatePlatformsBehaviour _manager_2 true true)
      (Default|UpdatePlatformsBehaviour _manager_2 false false)))
  (Default|UpdateBoozerColor _manager (Variables|/Game/Blueprints/GameModes/GM_LevelManager.GM_LevelManager_C|GetcurrentColor _manager)))