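; Inverter actor that swaps a set of linked platforms between red and blue.
; Its interaction zone registers it as the nearest inverter on BP_Boozer and toggles that character's ability to interact.
; InvertColors flips each platform, then has GM_LevelManager reapply the Boozer's current vision.
; Debug line traces show the links, colored by platform in construction and drawn every tick during normal vision.
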(event OnComponentBeginOverlap(InteractionZone)
  (params (OverlappedComponent :type Primitive%20Component%20Object%20Reference) (OtherActor :type Actor%20Object%20Reference) (OtherComp :type Primitive%20Component%20Object%20Reference) (OtherBodyIndex :type Integer) (bFromSweep :type Boolean) (SweepResult :type Hit%20Result%20Structure%20%28by%20ref%29))
  ;[1 1 1] Collision detector
  (bind _asbp_boozer (Utilities|Casting|CastToBP_Boozer OtherActor))
  (Variables|/Game/Blueprints/BP_Boozer.BP_Boozer_C|SetcanInteract _asbp_boozer true)
  (Variables|/Game/Blueprints/BP_Boozer.BP_Boozer_C|SetinteractionType _asbp_boozer "NewEnumerator1")
  (Variables|/Game/Blueprints/BP_Boozer.BP_Boozer_C|SetnearestInverter _asbp_boozer self))

(event OnComponentEndOverlap(InteractionZone)
  (params (OverlappedComponent :type Primitive%20Component%20Object%20Reference) (OtherActor :type Actor%20Object%20Reference) (OtherComp :type Primitive%20Component%20Object%20Reference) (OtherBodyIndex :type Integer))
  ;[1 1 1] Collision detector
  (bind _asbp_boozer (Utilities|Casting|CastToBP_Boozer OtherActor))
  (Variables|/Game/Blueprints/BP_Boozer.BP_Boozer_C|SetcanInteract _asbp_boozer false)
  (Variables|/Game/Blueprints/BP_Boozer.BP_Boozer_C|SetinteractionType _asbp_boozer "NewEnumerator0"))

(event EventBeginPlay
  (bind _returnvalue (Actor|GetActorOfClass "/Game/Blueprints/BP_Boozer.BP_Boozer_C"))
  (Variables|Default|SetboozerObj _returnvalue))

(event EventTick
  (params (DeltaSeconds :type Float%20%28single-precision%29))
  (bind _debugcolor (Variables|Default|GetdebugColor))
  (bind _debugcolor_2 (Variables|Default|GetdebugColor))
  ;[0.1838 0 0.3229] Pointer
  (switch Utilities|FlowControl|Switch|SwitchonVisionType (Variables|/Game/Blueprints/BP_Boozer.BP_Boozer_C|GetcurrentVisionType (Variables|Default|GetboozerObj))
    (:NewEnumerator0
      (for _array_element (Variables|Default|GetplatformsToInvert)
        (switch Utilities|FlowControl|Switch|SwitchonPlatformColor (Variables|/Game/Blueprints/GameLlements/BP_Platform.BP_Platform_C|GetcurrentColor _array_element)
          (:NewEnumerator1
            (Collision|LineTraceByChannel (Transformation|GetActorLocation) (Transformation|GetActorLocation _array_element) "TraceTypeQuery1" false 0 "ForOneFrame" true _debugcolor_2 _debugcolor_2))
          (:NewEnumerator2
            (Collision|LineTraceByChannel (Transformation|GetActorLocation) (Transformation|GetActorLocation _array_element) "TraceTypeQuery1" false 0 "ForOneFrame" true _debugcolor _debugcolor)))))))

(fn ConstructionScript
  (bind _returnvalue (Transformation|GetActorLocation))
  (for _array_element (Variables|Default|GetplatformsToInvert)
    (switch Utilities|FlowControl|Switch|SwitchonPlatformColor (Variables|/Game/Blueprints/GameLlements/BP_Platform.BP_Platform_C|GetcurrentColor _array_element)
      (:NewEnumerator1
        (Collision|LineTraceByChannel _returnvalue (Transformation|GetActorLocation _array_element) "TraceTypeQuery1" false 0 "ForDuration" true "(R=1.000000,G=0.000000,B=0.016807,A=1.000000)" "(R=1.000000,G=0.000000,B=0.016666,A=1.000000)"))
      (:NewEnumerator2
        (Collision|LineTraceByChannel _returnvalue (Transformation|GetActorLocation _array_element) "TraceTypeQuery1" false 0 "ForDuration" true "(R=0.000000,G=0.283149,B=1.000000,A=1.000000)" "(R=0.000000,G=0.283333,B=1.000000,A=1.000000)")))))

(fn InvertColors
  (for _array_element (Variables|Default|GetplatformsToInvert)
    (bind _output_get (LocalVariables|SetcurrentPlatform _array_element))
    (switch Utilities|FlowControl|Switch|SwitchonPlatformColor (Variables|/Game/Blueprints/GameLlements/BP_Platform.BP_Platform_C|GetcurrentColor _output_get) ; Check its current color to change it.
      (:NewEnumerator1
        (bind _output_get_2 (Variables|/Game/Blueprints/GameLlements/BP_Platform.BP_Platform_C|SetcurrentColor (LocalVariables|GetcurrentPlatform) "NewEnumerator2")) ; Red --> Blue
        (Default|UpdateColor (LocalVariables|GetcurrentPlatform) _output_get_2))
      (:NewEnumerator2
        (bind _output_get_3 (Variables|/Game/Blueprints/GameLlements/BP_Platform.BP_Platform_C|SetcurrentColor (LocalVariables|GetcurrentPlatform) "NewEnumerator1")) ; Blue --> Red
        (Default|UpdateColor (LocalVariables|GetcurrentPlatform) _output_get_3)))
    (bind _asgm_level_manager (Utilities|Casting|CastToGM_LevelManager (Game|GetGameMode)))
    (Default|UpdateBoozerVision _asgm_level_manager (Variables|/Game/Blueprints/BP_Boozer.BP_Boozer_C|GetcurrentVisionType (Variables|Default|GetboozerObj))) ; We must have in mind the current Boozer's vision.
  ))