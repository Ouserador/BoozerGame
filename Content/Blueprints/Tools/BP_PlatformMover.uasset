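; BP_PlatformMover is an interactable stone that toggles whether its linked MovablePlatforms can move.
; Its InteractionZone sets the interaction type on BP_Boozer and registers itself as NearestMover.
; AlterMover flips each platform's IsMovable and swaps the stone's pillar material to match.
; Debug line traces draw links to the platforms, color-coded by platform color at construction and every tick during the player's NORMAL vision.
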(event OnComponentBeginOverlap(InteractionZone)
  (params (OverlappedComponent :type Primitive%20Component%20Object%20Reference) (OtherActor :type Actor%20Object%20Reference) (OtherComp :type Primitive%20Component%20Object%20Reference) (OtherBodyIndex :type Integer) (bFromSweep :type Boolean) (SweepResult :type Hit%20Result%20Structure%20%28by%20ref%29))
  (bind _asbp_boozer (Utilities|Casting|CastToBP_Boozer OtherActor))
  (Variables|/Game/Blueprints/BP_Boozer.BP_Boozer_C|SetcanInteract _asbp_boozer true)
  (Variables|/Game/Blueprints/BP_Boozer.BP_Boozer_C|SetinteractionType _asbp_boozer "NewEnumerator2")
  (Variables|/Game/Blueprints/BP_Boozer.BP_Boozer_C|SetnearestMover _asbp_boozer self))

(event OnComponentEndOverlap(InteractionZone)
  (params (OverlappedComponent :type Primitive%20Component%20Object%20Reference) (OtherActor :type Actor%20Object%20Reference) (OtherComp :type Primitive%20Component%20Object%20Reference) (OtherBodyIndex :type Integer))
  (bind _asbp_boozer (Utilities|Casting|CastToBP_Boozer OtherActor))
  (Variables|/Game/Blueprints/BP_Boozer.BP_Boozer_C|SetcanInteract _asbp_boozer true)
  (Variables|/Game/Blueprints/BP_Boozer.BP_Boozer_C|SetinteractionType _asbp_boozer "NewEnumerator0"))

(event EventBeginPlay
  (bind _returnvalue (Actor|GetActorOfClass "/Game/Blueprints/BP_Boozer.BP_Boozer_C"))
  (Variables|Default|SetboozerObj _returnvalue))

(event EventTick
  (params (DeltaSeconds :type Float%20%28single-precision%29))
  (bind _debugcolor (Variables|Default|GetDebugColor))
  (switch Utilities|FlowControl|Switch|SwitchonVisionType (Variables|/Game/Blueprints/BP_Boozer.BP_Boozer_C|GetcurrentVisionType (Variables|Default|GetboozerObj))
    (:NewEnumerator0
      (for _array_element (Variables|Default|GetmovablePlatforms)
        (Collision|LineTraceByChannel (+ (Transformation|GetWorldLocation (Variables|Default|GetStone)) (Math|Vector|MakeVector 0.0 0.0 2e+01)) (Transformation|GetActorLocation _array_element) "TraceTypeQuery1" false 0 "ForOneFrame" true _debugcolor _debugcolor)))))

(fn ConstructionScript
  (bind _stone (Variables|Default|GetStone))
  (bind _returnvalue (Transformation|GetWorldLocation _stone))
  (for _array_element (Variables|Default|GetmovablePlatforms)
    (switch Utilities|FlowControl|Switch|SwitchonPlatformColor (Variables|/Game/Blueprints/GameLlements/BP_Platform.BP_Platform_C|GetcurrentColor _array_element)
      (:NewEnumerator0
        (Collision|LineTraceByChannel _returnvalue (Transformation|GetActorLocation _array_element) "TraceTypeQuery1" false 0 "ForDuration" true "(R=1.000000,G=0.000000,B=0.866688,A=1.000000)" "(R=1.000000,G=0.000000,B=0.863157,A=1.000000)" 1.0))
      (:NewEnumerator1
        (Collision|LineTraceByChannel _returnvalue (Transformation|GetActorLocation _array_element) "TraceTypeQuery1" false 0 "ForDuration" true "(R=1.000000,G=0.000000,B=0.016807,A=1.000000)" "(R=1.000000,G=0.000000,B=0.016666,A=1.000000)"))
      (:NewEnumerator2
        (Collision|LineTraceByChannel "0, 0, 0" (Transformation|GetActorLocation _array_element) "TraceTypeQuery1" false 0 "ForOneFrame" true "(R=0.000000,G=0.283149,B=1.000000,A=1.000000)" "(R=0.000000,G=0.283333,B=1.000000,A=1.000000)" 1.0)))))

(fn AlterMover
  (bind _stone (Variables|Default|GetStone))
  (for _array_element (Variables|Default|GetmovablePlatforms)
    (bind _output_get (Variables|/Game/Blueprints/GameLlements/BP_Platform.BP_Platform_C|SetisMovable _array_element (not (Variables|/Game/Blueprints/GameLlements/BP_Platform.BP_Platform_C|GetisMovable _array_element))))
    (if _output_get
      (Rendering|Material|SetMaterial _stone 0 "/Game/Materials/StonePilars/M_StonePilar_Off.M_StonePilar_Off")
      (else
        (Rendering|Material|SetMaterial _stone 0 "/Game/Materials/StonePilars/MI_StonePilar_On.MI_StonePilar_On")))))