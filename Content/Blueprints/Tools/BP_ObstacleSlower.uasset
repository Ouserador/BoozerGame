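; Interactable stone pillar that temporarily slows a linked set of rotating obstacles.
; Its overlap zone registers it with BP_Boozer and shows a button widget; ObstacleHandler sets a reduced rotation speed and lit material.
; Tick feeds the countdown to the HUD timer, then restores default speeds and availability.
; Debug-drawn line traces show links to each obstacle, at construction and every frame during NORMAL vision.
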(event OnComponentBeginOverlap(InteractionZone)
  (params (OverlappedComponent :type Primitive%20Component%20Object%20Reference) (OtherActor :type Actor%20Object%20Reference) (OtherComp :type Primitive%20Component%20Object%20Reference) (OtherBodyIndex :type Integer) (bFromSweep :type Boolean) (SweepResult :type Hit%20Result%20Structure%20%28by%20ref%29))
  ;[0 0.03548 0.276] Collision detection, interaction & UI pop-up
  (bind _asbp_boozer (Utilities|Casting|CastToBP_Boozer OtherActor))
  (Variables|/Game/Blueprints/BP_Boozer.BP_Boozer_C|SetcanInteract _asbp_boozer true)
  (Variables|/Game/Blueprints/BP_Boozer.BP_Boozer_C|SetinteractionType _asbp_boozer "NewEnumerator3")
  (Variables|/Game/Blueprints/BP_Boozer.BP_Boozer_C|SetnearestSlower _asbp_boozer self)
  (Rendering|SetVisibility (Variables|Default|GetButtonPopUp) true false))

(event OnComponentEndOverlap(InteractionZone)
  (params (OverlappedComponent :type Primitive%20Component%20Object%20Reference) (OtherActor :type Actor%20Object%20Reference) (OtherComp :type Primitive%20Component%20Object%20Reference) (OtherBodyIndex :type Integer))
  ;[0 0.03548 0.276] Collision detection, interaction & UI pop-up
  (bind _asbp_boozer (Utilities|Casting|CastToBP_Boozer OtherActor))
  (Variables|/Game/Blueprints/BP_Boozer.BP_Boozer_C|SetcanInteract _asbp_boozer false)
  (Variables|/Game/Blueprints/BP_Boozer.BP_Boozer_C|SetinteractionType _asbp_boozer "NewEnumerator0")
  (Rendering|SetVisibility (Variables|Default|GetButtonPopUp) false false))

(event Custom|ObstacleHandler
  ;[0.4115 0.8362 1] Slow obstacle
  (if (not (Variables|Default|GetisSlowed))
    (for _array_element (Variables|Default|GetnumObstacles)
      (Variables|/Game/Blueprints/GameLlements/BP_Obstacle.BP_Obstacle_C|SetrotationSpeed _array_element 5e+01))
    (Rendering|Material|SetMaterial (Variables|Default|GetStone) 0 "/Game/Materials/StonePilars/MI_StonePilar_On.MI_StonePilar_On")
    (Default|IsInteractionAvailable (Variables|Default|GetstoneUI) false)
    (Variables|Default|SetisSlowed true)
    (Default|ObstacleTimerShowing (Variables|/Game/Blueprints/GameModes/GM_LevelManager.GM_LevelManager_C|GetplayerHUD (Variables|/Game/Blueprints/BP_Boozer.BP_Boozer_C|Getmanager (Variables|Default|GetboozerObj))) true)))

(event EventBeginPlay
  (bind _buttonpopup (Variables|Default|GetButtonPopUp))
  (Utilities|FlowControl|Sequence
    (:then_0
      (bind _returnvalue (Actor|GetActorOfClass "/Game/Blueprints/BP_Boozer.BP_Boozer_C"))
      (Variables|Default|SetboozerObj _returnvalue))
    (:then_1
      (Rendering|SetVisibility _buttonpopup false false)
      (bind _asui_stone (Utilities|Casting|CastToUI_Stone (UserInterface|GetWidget _buttonpopup)))
      (bind _output_get (Variables|Default|SetstoneUI _asui_stone))
      (Default|IsInteractionAvailable _output_get true))
    (:then_2
      (Variables|Default|SetdelayTimer (Variables|Default|GetdelayTime)))))

(event EventTick
  (params (DeltaSeconds :type Float%20%28single-precision%29))
  ;[0.1534 0 0.4062] Pointer & slower behaviour
  (Utilities|FlowControl|Sequence
    (:then_0
      (CallFunction|Pointer))
    (:then_1
      (if (Variables|Default|GetisSlowed)
        (bind _output_get (Variables|Default|SetdelayTimer (- (Variables|Default|GetdelayTimer) (Utilities|Time|GetWorldDeltaSeconds))))
        (Default|ObstacleTimerBehaviour (Variables|/Game/Blueprints/GameModes/GM_LevelManager.GM_LevelManager_C|GetplayerHUD (Variables|/Game/Blueprints/BP_Boozer.BP_Boozer_C|Getmanager (Variables|Default|GetboozerObj))) (/ _output_get (Variables|Default|GetdelayTime)))
        (if (<= (Variables|Default|GetdelayTimer) 0.0)
          (for _array_element (Variables|Default|GetnumObstacles)
            (Variables|/Game/Blueprints/GameLlements/BP_Obstacle.BP_Obstacle_C|SetrotationSpeed _array_element (Variables|/Game/Blueprints/GameLlements/BP_Obstacle.BP_Obstacle_C|GetdefaultSpeed _array_element)))
          (Variables|Default|SetisSlowed false)
          (Rendering|Material|SetMaterial (Variables|Default|GetStone) 0 "/Game/Materials/StonePilars/M_StonePilar_Off.M_StonePilar_Off")
          (Default|IsInteractionAvailable (Variables|Default|GetstoneUI) true)
          (Variables|Default|SetdelayTimer (Variables|Default|GetdelayTime))
          (Default|ObstacleTimerShowing (Variables|/Game/Blueprints/GameModes/GM_LevelManager.GM_LevelManager_C|GetplayerHUD (Variables|/Game/Blueprints/BP_Boozer.BP_Boozer_C|Getmanager (Variables|Default|GetboozerObj))) false))))))

(fn ConstructionScript
  (for _array_element (Variables|Default|GetnumObstacles)
    (Collision|LineTraceByChannel (+ (Transformation|GetWorldLocation (Variables|Default|GetStone)) (Math|Vector|MakeVector 0.0 0.0 2e+01)) (Transformation|GetActorLocation _array_element) "TraceTypeQuery1" false 0 "ForDuration" true "(R=1.000000,G=1.000000,B=1.000000,A=1.000000)" "(R=1.000000,G=1.000000,B=1.000000,A=1.000000)")))

(fn Pointer
  (switch Utilities|FlowControl|Switch|SwitchonVisionType (Variables|/Game/Blueprints/BP_Boozer.BP_Boozer_C|GetcurrentVisionType (Variables|Default|GetboozerObj))
    (:NewEnumerator0
      (for _array_element (Variables|Default|GetnumObstacles)
        (Collision|LineTraceByChannel (+ (Transformation|GetWorldLocation (Variables|Default|GetStone)) (Math|Vector|MakeVector 0.0 0.0 2e+01)) (Transformation|GetActorLocation _array_element) "TraceTypeQuery1" false 0 "ForOneFrame" true "(R=1.000000,G=1.000000,B=1.000000,A=1.000000)" "(R=1.000000,G=1.000000,B=1.000000,A=1.000000)")))))