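; BP_CollectibleBottle is a collectible bottle pickup that the BP_Boozer character gathers in each level.
; On BeginPlay it picks the bottle's material from the current level name, falling back to the first bottle material.
; Tick spins the mesh around its yaw at RotationSpeed.
; Overlapping the trigger capsule increments the player's picked-bottle count, updates and animates the HUD counter, then destroys the actor.
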(event OnComponentBeginOverlap(TriggerCapsule)
  (params (OverlappedComponent :type Primitive%20Component%20Object%20Reference) (OtherActor :type Actor%20Object%20Reference) (OtherComp :type Primitive%20Component%20Object%20Reference) (OtherBodyIndex :type Integer) (bFromSweep :type Boolean) (SweepResult :type Hit%20Result%20Structure%20%28by%20ref%29))
  ;[1 0.151 0.9237] Collision detection, counter increment & UI animation
  (bind _asbp_boozer (Utilities|Casting|CastToBP_Boozer OtherActor))
  (bind _result (Math|Integer|IncrementInt (Variables|/Game/Blueprints/BP_Boozer.BP_Boozer_C|GetnumBottlesPicked _asbp_boozer))
    (:%20%20
      (Default|UpdateBottlesPerLevelCounter (Variables|/Game/Blueprints/GameModes/GM_LevelManager.GM_LevelManager_C|GetplayerHUD (Variables|/Game/Blueprints/BP_Boozer.BP_Boozer_C|Getmanager _asbp_boozer)) _result)
      (Default|PlayBottleAnimation (Variables|/Game/Blueprints/GameModes/GM_LevelManager.GM_LevelManager_C|GetplayerHUD (Variables|/Game/Blueprints/BP_Boozer.BP_Boozer_C|Getmanager _asbp_boozer)))
      (Actor|DestroyActor))))

(event EventTick
  (params (DeltaSeconds :type Float%20%28single-precision%29))
  (bind _bottle (Variables|Default|GetBottle))
  (bind _relativerotation (Variables|/Script/Engine.SceneComponent|GetRelativeRotation _bottle))
  ;[1 1 1] Rotation animation
  (Transformation|SetRelativeRotation (Variables|Default|GetBottle) (Math|Rotator|MakeRotator (.roll _relativerotation) (.pitch _relativerotation) (+ (* DeltaSeconds (Variables|Default|GetrotationSpeed)) (.yaw _relativerotation))) false false))

(event EventBeginPlay
  (bind _bottle (Variables|Default|GetBottle))
  ;[1 0.5473 0.01173] Texture setter
  (bind _returnvalue (Game|GetCurrentLevelName true))
  (switch string _returnvalue
    (:Default
      (Rendering|Material|SetMaterial _bottle 0 "/Game/Materials/Collectible_Bottles/M_Collectible_Bottle_1.M_Collectible_Bottle_1"))
    (:Level_1
      (Rendering|Material|SetMaterial _bottle 0 "/Game/Materials/Collectible_Bottles/M_Collectible_Bottle_1.M_Collectible_Bottle_1"))
    (:Level_2
      (Rendering|Material|SetMaterial _bottle 0 "/Game/Materials/Collectible_Bottles/MI_Collectible_Bottle_2.MI_Collectible_Bottle_2"))
    (:Level_3
      (Rendering|Material|SetMaterial _bottle 0 "/Game/Materials/Collectible_Bottles/MI_Collectible_Bottle_3.MI_Collectible_Bottle_3"))
    (:Level_4
      (Rendering|Material|SetMaterial _bottle 0 "/Game/Materials/Collectible_Bottles/MI_Collectible_Bottle_4.MI_Collectible_Bottle_4"))))

(fn ConstructionScript)