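; Colored level platform, optionally moving, that enables player abilities when its color matches the one held by GM_LevelManager.
; UpdateColor sets materials and collision, making purple translucent and non-solid.
; On non-vertical platforms, detector overlaps grant double jump on red or flag the Boozer on blue, updating HUD text and hat glow.
; Movable platforms start at the spline's first point and copy SplinePath's reference point location every tick.
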(event OnComponentBeginOverlap(BoozerDetector)
  (params (OverlappedComponent :type Primitive%20Component%20Object%20Reference) (OtherActor :type Actor%20Object%20Reference) (OtherComp :type Primitive%20Component%20Object%20Reference) (OtherBodyIndex :type Integer) (bFromSweep :type Boolean) (SweepResult :type Hit%20Result%20Structure%20%28by%20ref%29))
  (bind _manager (Variables|Default|Getmanager))
  (bind _manager_2 (Variables|Default|Getmanager))
  (bind _manager_3 (Variables|Default|Getmanager))
  (bind _boozerobj (Variables|Default|GetboozerObj))
  (bind _isredcolor (Variables|/Game/Blueprints/GameModes/GM_LevelManager.GM_LevelManager_C|GetisRedColor _manager_2))
  (bind _hatobj (Variables|/Game/Blueprints/BP_Boozer.BP_Boozer_C|GethatObj _boozerobj))
  (bind _hat (Variables|/Game/Blueprints/BP_Hat.BP_Hat_C|GetHat _hatobj))
  ;[1 1 1] Red/Blue platform detection
  (bind _asbp_boozer (Utilities|Casting|CastToBP_Boozer OtherActor))
  (if (Variables|/Game/Blueprints/GameModes/GM_LevelManager.GM_LevelManager_C|GethasAbilities (Variables|Default|Getmanager))
    (if (not (Variables|Main|GetisVertical))
      (switch Utilities|FlowControl|Switch|SwitchonPlatformColor (Variables|Main|GetcurrentColor)
        (:NewEnumerator0
          (Variables|/Script/Engine.Character|SetJumpMaxCount (Variables|Default|GetboozerObj) 1 :!label _label)
          (Variables|/Script/Engine.CharacterMovementComponent|SetGravityScale (Variables|/Script/Engine.Character|GetCharacterMovement (Variables|Default|GetboozerObj)) 1.5)
          (switch Utilities|FlowControl|Switch|SwitchonColorType (Variables|/Game/Blueprints/GameModes/GM_LevelManager.GM_LevelManager_C|GetcurrentColor (Variables|Default|Getmanager))
            (:NewEnumerator0
              (Rendering|Material|SetMaterial _hat 0 "/Game/Materials/Hat/MI_Hat_Red.MI_Hat_Red"))
            (:NewEnumerator1
              (Rendering|Material|SetMaterial _hat 0 "/Game/Materials/Hat/MI_Hat_Blue.MI_Hat_Blue"))))
        (:NewEnumerator1
          (if _isredcolor
            (Variables|/Game/Blueprints/BP_Boozer.BP_Boozer_C|SetinRedPlatform _asbp_boozer true)
            (Variables|/Script/Engine.Character|SetJumpMaxCount (Variables|Default|GetboozerObj) 2)
            (Default|UpdateAbilityTxt (Variables|/Game/Blueprints/GameModes/GM_LevelManager.GM_LevelManager_C|GetplayerHUD _manager) true (Variables|/Game/Blueprints/GameModes/GM_LevelManager.GM_LevelManager_C|GetcurrentColor _manager))
            (Rendering|Material|SetMaterial (Variables|/Game/Blueprints/BP_Hat.BP_Hat_C|GetHat (Variables|/Game/Blueprints/BP_Boozer.BP_Boozer_C|GethatObj (Variables|Default|GetboozerObj))) 0 "/Game/Materials/Hat/MI_Hat_Glow_Red.MI_Hat_Glow_Red")
            (else
              (Variables|/Script/Engine.Character|SetJumpMaxCount (Variables|Default|GetboozerObj) 1))))
        (:NewEnumerator2
          (if _isredcolor
            (goto _label)
            (else
              (Variables|/Game/Blueprints/BP_Boozer.BP_Boozer_C|SetinBluePlatform _asbp_boozer true)
              (Default|UpdateAbilityTxt (Variables|/Game/Blueprints/GameModes/GM_LevelManager.GM_LevelManager_C|GetplayerHUD _manager_3) true (Variables|/Game/Blueprints/GameModes/GM_LevelManager.GM_LevelManager_C|GetcurrentColor _manager_3))
              (Rendering|Material|SetMaterial (Variables|/Game/Blueprints/BP_Hat.BP_Hat_C|GetHat (Variables|/Game/Blueprints/BP_Boozer.BP_Boozer_C|GethatObj (Variables|Default|GetboozerObj))) 0 "/Game/Materials/Hat/MI_Hat_Glow_Blue.MI_Hat_Glow_Blue"))))
        (:NewEnumerator3
          (goto _label))))))

(event OnComponentEndOverlap(BoozerDetector)
  (params (OverlappedComponent :type Primitive%20Component%20Object%20Reference) (OtherActor :type Actor%20Object%20Reference) (OtherComp :type Primitive%20Component%20Object%20Reference) (OtherBodyIndex :type Integer))
  (bind _boozerobj (Variables|Default|GetboozerObj))
  (bind _manager (Variables|Default|Getmanager))
  (bind _hatobj (Variables|/Game/Blueprints/BP_Boozer.BP_Boozer_C|GethatObj _boozerobj))
  (bind _currentcolor (Variables|/Game/Blueprints/GameModes/GM_LevelManager.GM_LevelManager_C|GetcurrentColor _manager))
  (bind _hat (Variables|/Game/Blueprints/BP_Hat.BP_Hat_C|GetHat _hatobj))
  ;[1 1 1] Red/Blue platform detection
  (bind _asbp_boozer (Utilities|Casting|CastToBP_Boozer OtherActor))
  (if (Variables|/Game/Blueprints/GameModes/GM_LevelManager.GM_LevelManager_C|GethasAbilities (Variables|Default|Getmanager))
    (if (not (Variables|Main|GetisVertical))
      (switch Utilities|FlowControl|Switch|SwitchonPlatformColor (Variables|Main|GetcurrentColor)
        (:NewEnumerator1
          (Variables|/Game/Blueprints/BP_Boozer.BP_Boozer_C|SetinRedPlatform _asbp_boozer false)
          (Rendering|Material|SetMaterial (Variables|/Game/Blueprints/BP_Hat.BP_Hat_C|GetHat (Variables|/Game/Blueprints/BP_Boozer.BP_Boozer_C|GethatObj (Variables|Default|GetboozerObj))) 0 "/Game/Materials/Hat/MI_Hat_Red.MI_Hat_Red"))
        (:NewEnumerator2
          (Variables|/Game/Blueprints/BP_Boozer.BP_Boozer_C|SetinBluePlatform _asbp_boozer false)
          (Rendering|Material|SetMaterial (Variables|/Game/Blueprints/BP_Hat.BP_Hat_C|GetHat (Variables|/Game/Blueprints/BP_Boozer.BP_Boozer_C|GethatObj (Variables|Default|GetboozerObj))) 0 "/Game/Materials/Hat/MI_Hat_Blue.MI_Hat_Blue")))
      (Default|UpdateAbilityTxt (Variables|/Game/Blueprints/GameModes/GM_LevelManager.GM_LevelManager_C|GetplayerHUD _manager) false _currentcolor)
      (switch Utilities|FlowControl|Switch|SwitchonColorType _currentcolor
        (:NewEnumerator0
          (Rendering|Material|SetMaterial _hat 0 "/Game/Materials/Hat/MI_Hat_Red.MI_Hat_Red"))
        (:NewEnumerator1
          (Rendering|Material|SetMaterial _hat 0 "/Game/Materials/Hat/MI_Hat_Blue.MI_Hat_Blue"))))))

(event Custom|MovePlatformThroughSpline
  (Transformation|SetActorLocation (Transformation|GetWorldLocation (Variables|/Game/Blueprints/GameLlements/BP_Spline.BP_Spline_C|GetRefPoint (Variables|Main|GetsplinePath))) false false))

(event EventBeginPlay
  (Utilities|FlowControl|Sequence
    (:then_0
      (bind _returnvalue (Actor|GetActorOfClass "/Game/Blueprints/BP_Boozer.BP_Boozer_C"))
      (Variables|Default|SetboozerObj _returnvalue))
    (:then_1
      (bind _asgm_level_manager (Utilities|Casting|CastToGM_LevelManager (Game|GetGameMode)))
      (Variables|Default|Setmanager _asgm_level_manager))))

(event EventTick
  (params (DeltaSeconds :type Float%20%28single-precision%29))
  (bind _splinepath (Variables|Main|GetsplinePath))
  (if (Variables|Main|GetisMovable)
    (Variables|/Game/Blueprints/GameLlements/BP_Spline.BP_Spline_C|SetallowMovement (Variables|Main|GetsplinePath) true) ; Move the ref. point...
    (CallFunction|MovePlatformThroughSpline) ; ...then the platform.
    (else
      (Utilities|IsValid _splinepath ; No all platforms have this component. It has to be checked.
        (:Is%20Valid
          (Variables|/Game/Blueprints/GameLlements/BP_Spline.BP_Spline_C|SetallowMovement _splinepath false))))))

(fn ConstructionScript
  (Utilities|FlowControl|Sequence
    (:then_0
      (CallFunction|UpdateColor (Variables|Main|GetcurrentColor)))
    (:then_1
      (if (Variables|Main|GetisMovable)
        (Transformation|SetActorLocation (Spline|GetLocationatSplinePoint (Variables|/Game/Blueprints/GameLlements/BP_Spline.BP_Spline_C|GetSpline (Variables|Main|GetsplinePath)) 0 "World") false false)))))

(fn UpdateColor
  (params (newColor :type PlatformColor%20Enum :default "NewEnumerator0"))
  (switch Utilities|FlowControl|Switch|SwitchonPlatformColor newColor
    (:NewEnumerator0
      (CallFunction|ChangeProperties "/Game/Materials/Platforms/M_Platform.M_Platform" true))
    (:NewEnumerator1
      (CallFunction|ChangeProperties "/Game/Materials/Platforms/MI_Platform_Red.MI_Platform_Red" true))
    (:NewEnumerator2
      (CallFunction|ChangeProperties "/Game/Materials/Platforms/MI_Platform_Blue.MI_Platform_Blue" true))
    (:NewEnumerator3
      (CallFunction|ChangeProperties "/Game/Materials/Platforms/M_PlatformTranslucent_Purple.M_PlatformTranslucent_Purple" false)))
  (Rendering|Material|SetMaterial (Variables|Default|GetRopes) 0 "/Game/Materials/Platforms/M_Rope.M_Rope"))

(fn ChangeProperties
  (params (newColorMat :type Material%20Interface%20Object%20Reference) (hasCollision :type Boolean))
  (bind _boozerdetector (Variables|Default|GetBoozerDetector))
  (bind _mesh (Variables|Default|GetMesh))
  (Utilities|FlowControl|Sequence
    (:then_0
      (Rendering|Material|SetMaterial (Variables|Default|GetMesh) 0 newColorMat) ; Change material.
    )
    (:then_1
      (if hasCollision
        (Collision|SetCollisionEnabled _mesh "QueryAndPhysics")
        (Variables|Default|SetisTransparent false)
        (Rendering|Material|SetMaterial (Variables|Default|GetRopes) 0 "/Game/Materials/Platforms/M_Rope.M_Rope")
        (Collision|SetCollisionEnabled _boozerdetector "QueryAndPhysics")
        (else
          (Collision|SetCollisionEnabled _mesh "NoCollision")
          (Variables|Default|SetisTransparent true)
          (Rendering|Material|SetMaterial (Variables|Default|GetRopes) 0 "/Game/Materials/Platforms/M_RopeTranslucent.M_RopeTranslucent")
          (Collision|SetCollisionEnabled _boozerdetector "NoCollision"))))))