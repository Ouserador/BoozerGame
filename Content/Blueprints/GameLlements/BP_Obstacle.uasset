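; BP_Obstacle is a spinning obstacle actor that shoves boozer characters on contact.
; It sets its rotation speed from a default on BeginPlay and advances its yaw every Tick, scaled by delta time.
; When its collider hits a BP_Boozer, it sends a fixed-strength push along the obstacle's right vector to that boozer and plays a collision sound.
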(event OnComponentHit(Collider)
  (params (HitComponent :type Primitive%20Component%20Object%20Reference) (OtherActor :type Actor%20Object%20Reference) (OtherComp :type Primitive%20Component%20Object%20Reference) (NormalImpulse :type Vector :default "0, 0, 0") (Hit :type Hit%20Result%20Structure%20%28by%20ref%29))
  ;[1 0.2321 0] Push Boozer
  (bind _asbp_boozer (Utilities|Casting|CastToBP_Boozer OtherActor))
  (Default|OnBeingPushedbyObstacle _asbp_boozer (* (Transformation|GetActorRightVector) 1e+03))
  (Audio|PlaySoundatLocation "/Game/Audio/Sounds/Obstacle/obstacle_collision.obstacle_collision" (Transformation|GetActorLocation) "0, 0, 0" 1.0 1.0 0.0 0 0 0 0))

(event EventTick
  (params (DeltaSeconds :type Float%20%28single-precision%29))
  ;[0 0.2482 0.5781] Rotation
  (Transformation|SetActorRotation (Math|Rotator|MakeRotator 0.0 0.0 (+ (* (Variables|Default|GetrotationSpeed) (Utilities|Time|GetWorldDeltaSeconds)) (.yaw (Transformation|GetActorRotation))))))

(event EventBeginPlay
  (Variables|Default|SetrotationSpeed (Variables|Default|GetdefaultSpeed)))

(fn ConstructionScript)