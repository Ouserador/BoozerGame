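; Game mode that manages a level's red/blue platform vision mechanic, HUD and Boozer respawns.
; BeginPlay applies saved colorblind settings, creates the HUD, caches level actors and adds the bottle count to the game instance.
; Vision changes make platforms solid or non-colliding translucent, with the current color deciding which translucent ones stay visible.
; OnDying respawns Boozer at the start or matching checkpoint, and first Tick forces red vision as a bug workaround.
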(event Custom|OnDying
  (bind _boozerobj (Variables|Default|GetboozerObj))
  (bind _boozerobj_2 (Variables|Default|GetboozerObj))
  (bind _boozerobj_3 (Variables|Default|GetboozerObj))
  (bind _startposobj (Variables|Default|GetstartPosObj))
  (bind _returnvalue (Transformation|GetActorTransform _startposobj))
  ;[0.6094 0.02856 0.02856] Boozer's death and respawn
  (if (!= (Variables|/Game/Blueprints/BP_Boozer.BP_Boozer_C|GetcurrentCheckpoint _boozerobj_3) 0)
    (for _array_element (Variables|Default|GetnumCheckpoints) ; Check every checkpoint.
      (if (== (Variables|/Game/Blueprints/LevelElements/BP_Checkpoint.BP_Checkpoint_C|GetcheckPointValue _array_element) (Variables|/Game/Blueprints/BP_Boozer.BP_Boozer_C|GetcurrentCheckpoint _boozerobj_2))
        (if (Variables|/Game/Blueprints/LevelElements/BP_Checkpoint.BP_Checkpoint_C|GetdoubleColor _array_element)
          (if (Utilities|Enum|Equal(Enum) (Variables|/Game/Blueprints/LevelElements/BP_Checkpoint.BP_Checkpoint_C|GetcolorType _array_element) (Variables|GM_LevelManager_C|GetcurrentColor (Variables|/Game/Blueprints/BP_Boozer.BP_Boozer_C|Getmanager _boozerobj_2)))
            (Transformation|SetActorTransform _boozerobj (Math|Transform|MakeTransform (.location (Transformation|GetWorldTransform (Variables|/Game/Blueprints/LevelElements/BP_Checkpoint.BP_Checkpoint_C|GetSpawnPoint _array_element))) (.rotation (Transformation|GetWorldTransform (Variables|/Game/Blueprints/LevelElements/BP_Checkpoint.BP_Checkpoint_C|GetSpawnPoint _array_element))) "1.000000,1.000000,1.000000") :!label _label) ; Boozer respawns at the last checkpoint.
            (Variables|/Script/Engine.MovementComponent|SetVelocity (Variables|/Script/Engine.Character|GetCharacterMovement _boozerobj) "0, 0, 0") ; Respawning with no velocity.
          )
          (else
            (goto _label)))))
    (else
      (Transformation|SetActorTransform _boozerobj_3 (Math|Transform|MakeTransform (.location _returnvalue) (.rotation _returnvalue) "1.000000,1.000000,1.000000")) ; Boozer respawns at the beginning.
      (Variables|/Script/Engine.MovementComponent|SetVelocity (Variables|/Script/Engine.Character|GetCharacterMovement _boozerobj) "0, 0, 0") ; Respawning with no velocity.
    )))

(event EventBeginPlay
  (Utilities|FlowControl|Sequence
    (:then_0
      (CallFunction|SetPlatformArray)
      (bind _asgi_instance (Utilities|Casting|CastToGI_Instance (Game|GetGameInstance)))
      (bind _output_get (Variables|Default|Setinstance _asgi_instance))
      (bind (_cbtype _cbstrenght) (Default|GetValues _output_get)) ; Firstly, update the values and set them in the current level.
      (switch Utilities|FlowControl|Switch|SwitchonColorBlindType _cbtype
        (:NewEnumerator0
          (Class|WidgetBlueprintLibrary|SetColorVisionDeficiencyType "NormalVision" _cbstrenght true true))
        (:NewEnumerator1
          (Class|WidgetBlueprintLibrary|SetColorVisionDeficiencyType "Deuteranope" _cbstrenght true true))
        (:NewEnumerator2
          (Class|WidgetBlueprintLibrary|SetColorVisionDeficiencyType "Protanope" _cbstrenght true true))
        (:NewEnumerator3
          (Class|WidgetBlueprintLibrary|SetColorVisionDeficiencyType "Tritanope" _cbstrenght true true))))
    (:then_1
      (CallFunction|InitHUD "NewEnumerator2")
      (Default|UpdateBottlesPerLevelCounter (Variables|Default|GetplayerHUD)))
    (:then_2
      (bind _returnvalue (Actor|GetActorOfClass "/Game/Blueprints/BP_Boozer.BP_Boozer_C"))
      (Variables|Default|SetboozerObj _returnvalue))
    (:then_3
      (bind _outactors (Actor|GetAllActorsOfClass "/Game/Blueprints/LevelElements/BP_Checkpoint.BP_Checkpoint_C"))
      (Variables|Default|SetnumCheckpoints _outactors))
    (:then_4
      (bind _returnvalue_2 (Actor|GetActorOfClass "/Game/Blueprints/LevelElements/BP_StartPosition.BP_StartPosition_C"))
      (Variables|Default|SetstartPosObj _returnvalue_2))
    (:then_5
      (bind _outactors_2 (Actor|GetAllActorsOfClass "/Game/Blueprints/GameLlements/BP_CollectibleBottle.BP_CollectibleBottle_C"))
      (bind _output_get_2 (Variables|Default|SetnumCollectiblesAtLvl (Utilities|Array|Length _outactors_2)))
      (Default|SetMaxCollectibles (Variables|Default|Getinstance) _output_get_2) ; Add the current number of collectibles in the current level to the counter.
    )))

(event EventTick
  (params (DeltaSeconds :type Float%20%28single-precision%29))
  (if (Variables|Default|GetisFirstTime)
    (bind _output_get (Variables|/Game/Blueprints/BP_Boozer.BP_Boozer_C|SetcurrentVisionType (Variables|Default|GetboozerObj) "NewEnumerator1"))
    (CallFunction|UpdateBoozerVision _output_get)
    (Variables|Default|SetisFirstTime false)))

(fn ConstructionScript)

(fn SetPlatformArray
  (bind _outactors (Actor|GetAllActorsOfClass "/Game/Blueprints/GameLlements/BP_Platform.BP_Platform_C")) ; Get all platforms in the level.
  (Variables|PlatformArrays|SetnumPlatforms _outactors))

(fn UpdateBoozerVision
  (params (newVision :type VisionType%20Enum :default "NewEnumerator0"))
  (bind _playerhud (Variables|Default|GetplayerHUD))
  (switch Utilities|FlowControl|Switch|SwitchonVisionType newVision
    (:NewEnumerator0
      (Default|UpdateVisionSelector _playerhud "NewEnumerator0")
      (CallFunction|UpdatePlatformsBehaviour true true)
      (CallFunction|UpdatePlatformsBehaviour false true))
    (:NewEnumerator1
      (Default|UpdateVisionSelector _playerhud "NewEnumerator1")
      (CallFunction|UpdatePlatformsBehaviour true false)
      (CallFunction|UpdatePlatformsBehaviour false true))
    (:NewEnumerator2
      (Default|UpdateVisionSelector _playerhud "NewEnumerator2")
      (CallFunction|UpdatePlatformsBehaviour true true)
      (CallFunction|UpdatePlatformsBehaviour false false))))

(fn UpdatePlatformsBehaviour
  (params (isRed :type Boolean) (isTranslucent :type Boolean))
  (if isRed ; Red or Blue
    (for _array_element (Variables|PlatformArrays|GetnumPlatforms)
      (switch Utilities|FlowControl|Switch|SwitchonPlatformColor (Variables|/Game/Blueprints/GameLlements/BP_Platform.BP_Platform_C|GetcurrentColor _array_element)
        (:NewEnumerator1
          (if isTranslucent
            (switch Utilities|FlowControl|Switch|SwitchonColorType (Variables|Default|GetcurrentColor)
              (:NewEnumerator0
                (Default|ChangeProperties _array_element "/Game/Materials/Platforms/M_PlatformTranslucent_Red.M_PlatformTranslucent_Red" false)
                (Rendering|SetVisibility (Variables|/Game/Blueprints/GameLlements/BP_Platform.BP_Platform_C|GetMesh _array_element) true false)
                (Rendering|SetVisibility (Variables|/Game/Blueprints/GameLlements/BP_Platform.BP_Platform_C|GetRopes _array_element) true false))
              (:NewEnumerator1
                (Default|ChangeProperties _array_element "/Game/Materials/Platforms/M_PlatformTranslucent_Red.M_PlatformTranslucent_Red" false)
                (Rendering|SetVisibility (Variables|/Game/Blueprints/GameLlements/BP_Platform.BP_Platform_C|GetMesh _array_element) false false)
                (Rendering|SetVisibility (Variables|/Game/Blueprints/GameLlements/BP_Platform.BP_Platform_C|GetRopes _array_element) false false)))
            (else
              (Default|ChangeProperties _array_element "/Game/Materials/Platforms/MI_Platform_Red.MI_Platform_Red" true)
              (Rendering|SetVisibility (Variables|/Game/Blueprints/GameLlements/BP_Platform.BP_Platform_C|GetMesh _array_element) true false)
              (Rendering|SetVisibility (Variables|/Game/Blueprints/GameLlements/BP_Platform.BP_Platform_C|GetRopes _array_element) true false))))))
    (else
      (for _array_element_2 (Variables|PlatformArrays|GetnumPlatforms)
        (switch Utilities|FlowControl|Switch|SwitchonPlatformColor (Variables|/Game/Blueprints/GameLlements/BP_Platform.BP_Platform_C|GetcurrentColor _array_element_2)
          (:NewEnumerator2
            (if isTranslucent
              (switch Utilities|FlowControl|Switch|SwitchonColorType (Variables|Default|GetcurrentColor)
                (:NewEnumerator0
                  (Default|ChangeProperties _array_element_2 "/Game/Materials/Platforms/MI_PlatformTranslucent_Blue.MI_PlatformTranslucent_Blue" false)
                  (Rendering|SetVisibility (Variables|/Game/Blueprints/GameLlements/BP_Platform.BP_Platform_C|GetMesh _array_element_2) false false)
                  (Rendering|SetVisibility (Variables|/Game/Blueprints/GameLlements/BP_Platform.BP_Platform_C|GetRopes _array_element_2) false false))
                (:NewEnumerator1
                  (Default|ChangeProperties _array_element_2 "/Game/Materials/Platforms/MI_PlatformTranslucent_Blue.MI_PlatformTranslucent_Blue" false)
                  (Rendering|SetVisibility (Variables|/Game/Blueprints/GameLlements/BP_Platform.BP_Platform_C|GetMesh _array_element_2) true false)
                  (Rendering|SetVisibility (Variables|/Game/Blueprints/GameLlements/BP_Platform.BP_Platform_C|GetRopes _array_element_2) true false)))
              (else
                (Default|ChangeProperties _array_element_2 "/Game/Materials/Platforms/MI_Platform_Blue.MI_Platform_Blue" true)
                (Rendering|SetVisibility (Variables|/Game/Blueprints/GameLlements/BP_Platform.BP_Platform_C|GetMesh _array_element_2) true false)
                (Rendering|SetVisibility (Variables|/Game/Blueprints/GameLlements/BP_Platform.BP_Platform_C|GetRopes _array_element_2) true false)))))))))

(fn InitHUD
  (params (color :type ColorType%20Enum :default "NewEnumerator0"))
  (bind _returnvalue (Game|GetPlayerController 0))
  (Variables|Default|SetcurrentColor color)
  (bind _returnvalue_2 (UserInterface|CreateWidget "/Game/UI/UI_PlayerHUD.UI_PlayerHUD_C" _returnvalue))
  (bind _output_get (Variables|Default|SetplayerHUD _returnvalue_2))
  (UserInterface|Viewport|AddtoViewport _output_get 0)
  (Input|SetInputModeGameOnly _returnvalue false)
  (Variables|/Script/Engine.PlayerController|SetbShowMouseCursor _returnvalue false)
  (Default|SetCurrentColorImg (Variables|Default|GetplayerHUD) (Variables|Default|GetcurrentColor))
  (Default|UpdateAbilityTxt (Variables|Default|GetplayerHUD) false (Variables|Default|GetcurrentColor))
  (switch Utilities|FlowControl|Switch|SwitchonColorType (Variables|Default|GetcurrentColor)
    (:NewEnumerator2
      (Variables|Default|SethasAbilities false))
    (:NewEnumerator0
      (Variables|Default|SetisRedColor true))
    (:NewEnumerator1
      (Variables|Default|SetisRedColor false))))

(fn UpdateBoozerColor
  (params (newColor :type ColorType%20Enum :default "NewEnumerator0"))
  (Default|SetCurrentColorImg (Variables|Default|GetplayerHUD) newColor)
  (bind _returnvalue (Actor|GetActorOfClass "/Game/Blueprints/BP_Hat.BP_Hat_C"))
  (Default|UpdateHatColor _returnvalue newColor))